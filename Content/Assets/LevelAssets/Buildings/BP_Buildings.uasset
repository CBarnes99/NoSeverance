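; Configurable building prop for level dressing that swaps its static mesh and color material from two enum selections.
; The construction script runs SetMesh to pick one of many one- to six-story building variants from Buildings, then SetMaterial to apply the chosen material instance to slot 0.
; It then forces the mesh's world scale to a uniform 3x.
; The event graph is empty, so it has no runtime logic.
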(event EventBeginPlay)

(event Collision|EventActorBeginOverlap
  (params (OtherActor :type Actor%20Object%20Reference)))

(event EventTick
  (params (DeltaSeconds :type Float%20%28single-precision%29)))

(fn ConstructionScript
  (CallFunction|SetMesh)
  (CallFunction|SetMaterial)
  (Transformation|SetWorldScale3D (Variables|Default|GetStaticMesh) "3.000000,3.000000,3.000000"))

(fn SetMesh
  (switch Utilities|FlowControl|Switch|SwitchonE_Buildings (Variables|Default|GetBuildings)
    (:NewEnumerator3
      (Components|StaticMesh|SetStaticMesh (Variables|Default|GetStaticMesh) "/Game/Assets/LevelAssets/Buildings/StaticMeshes/1Story.1Story"))
    (:NewEnumerator4
      (Components|StaticMesh|SetStaticMesh (Variables|Default|GetStaticMesh) "/Game/Assets/LevelAssets/Buildings/StaticMeshes/1Story_GableRoof.1Story_GableRoof"))
    (:NewEnumerator5
      (Components|StaticMesh|SetStaticMesh (Variables|Default|GetStaticMesh) "/Game/Assets/LevelAssets/Buildings/StaticMeshes/1Story_RoundRoof.1Story_RoundRoof"))
    (:NewEnumerator6
      (Components|StaticMesh|SetStaticMesh (Variables|Default|GetStaticMesh) "/Game/Assets/LevelAssets/Buildings/StaticMeshes/1Story_Sign.1Story_Sign"))
    (:NewEnumerator7
      (Components|StaticMesh|SetStaticMesh (Variables|Default|GetStaticMesh) "/Game/Assets/LevelAssets/Buildings/StaticMeshes/2Story.2Story"))
    (:NewEnumerator8
      (Components|StaticMesh|SetStaticMesh (Variables|Default|GetStaticMesh) "/Game/Assets/LevelAssets/Buildings/StaticMeshes/2Story_2.2Story_2"))
    (:NewEnumerator9
      (Components|StaticMesh|SetStaticMesh (Variables|Default|GetStaticMesh) "/Game/Assets/LevelAssets/Buildings/StaticMeshes/2Story_Balcony.2Story_Balcony"))
    (:NewEnumerator10
      (Components|StaticMesh|SetStaticMesh (Variables|Default|GetStaticMesh) "/Game/Assets/LevelAssets/Buildings/StaticMeshes/2Story_Center.2Story_Center"))
    (:NewEnumerator11
      (Components|StaticMesh|SetStaticMesh (Variables|Default|GetStaticMesh) "/Game/Assets/LevelAssets/Buildings/StaticMeshes/2Story_Columns.2Story_Columns"))
    (:NewEnumerator12
      (Components|StaticMesh|SetStaticMesh (Variables|Default|GetStaticMesh) "/Game/Assets/LevelAssets/Buildings/StaticMeshes/2Story_Double.2Story_Double"))
    (:NewEnumerator13
      (Components|StaticMesh|SetStaticMesh (Variables|Default|GetStaticMesh) "/Game/Assets/LevelAssets/Buildings/StaticMeshes/2Story_GableRoof.2Story_GableRoof"))
    (:NewEnumerator14
      (Components|StaticMesh|SetStaticMesh (Variables|Default|GetStaticMesh) "/Game/Assets/LevelAssets/Buildings/StaticMeshes/2Story_RoundRoof.2Story_RoundRoof"))
    (:NewEnumerator15
      (Components|StaticMesh|SetStaticMesh (Variables|Default|GetStaticMesh) "/Game/Assets/LevelAssets/Buildings/StaticMeshes/2Story_Sidehouse.2Story_Sidehouse"))
    (:NewEnumerator16
      (Components|StaticMesh|SetStaticMesh (Variables|Default|GetStaticMesh) "/Game/Assets/LevelAssets/Buildings/StaticMeshes/2Story_Sign.2Story_Sign"))
    (:NewEnumerator17
      (Components|StaticMesh|SetStaticMesh (Variables|Default|GetStaticMesh) "/Game/Assets/LevelAssets/Buildings/StaticMeshes/2Story_Slim.2Story_Slim"))
    (:NewEnumerator18
      (Components|StaticMesh|SetStaticMesh (Variables|Default|GetStaticMesh) "/Game/Assets/LevelAssets/Buildings/StaticMeshes/2Story_Stairs.2Story_Stairs"))
    (:NewEnumerator19
      (Components|StaticMesh|SetStaticMesh (Variables|Default|GetStaticMesh) "/Game/Assets/LevelAssets/Buildings/StaticMeshes/2Story_Wide.2Story_Wide"))
    (:NewEnumerator20
      (Components|StaticMesh|SetStaticMesh (Variables|Default|GetStaticMesh) "/Game/Assets/LevelAssets/Buildings/StaticMeshes/2Story_Wide_2Doors.2Story_Wide_2Doors"))
    (:NewEnumerator21
      (Components|StaticMesh|SetStaticMesh (Variables|Default|GetStaticMesh) "/Game/Assets/LevelAssets/Buildings/StaticMeshes/3Story_Balcony.3Story_Balcony"))
    (:NewEnumerator22
      (Components|StaticMesh|SetStaticMesh (Variables|Default|GetStaticMesh) "/Game/Assets/LevelAssets/Buildings/StaticMeshes/3Story_Slim.3Story_Slim"))
    (:NewEnumerator23
      (Components|StaticMesh|SetStaticMesh (Variables|Default|GetStaticMesh) "/Game/Assets/LevelAssets/Buildings/StaticMeshes/3Story_Small.3Story_Small"))
    (:NewEnumerator24
      (Components|StaticMesh|SetStaticMesh (Variables|Default|GetStaticMesh) "/Game/Assets/LevelAssets/Buildings/StaticMeshes/4Story.4Story"))
    (:NewEnumerator25
      (Components|StaticMesh|SetStaticMesh (Variables|Default|GetStaticMesh) "/Game/Assets/LevelAssets/Buildings/StaticMeshes/4Story_Center.4Story_Center"))
    (:NewEnumerator26
      (Components|StaticMesh|SetStaticMesh (Variables|Default|GetStaticMesh) "/Game/Assets/LevelAssets/Buildings/StaticMeshes/4Story_Wide_2Doors.4Story_Wide_2Doors"))
    (:NewEnumerator27
      (Components|StaticMesh|SetStaticMesh (Variables|Default|GetStaticMesh) "/Game/Assets/LevelAssets/Buildings/StaticMeshes/4Story_Wide_2Doors_Roof.4Story_Wide_2Doors_Roof"))
    (:NewEnumerator28
      (Components|StaticMesh|SetStaticMesh (Variables|Default|GetStaticMesh) "/Game/Assets/LevelAssets/Buildings/StaticMeshes/6Story_Stack.6Story_Stack"))))

(fn SetMaterial
  (switch Utilities|FlowControl|Switch|SwitchonE_BuildingMaterial (Variables|Default|GetMaterials)
    (:NewEnumerator0
      (Rendering|Material|SetMaterial (Variables|Default|GetStaticMesh) 0 "/Game/Assets/LevelAssets/Buildings/Materials/MI_BuildingTexture_Blue.MI_BuildingTexture_Blue"))
    (:NewEnumerator1
      (Rendering|Material|SetMaterial (Variables|Default|GetStaticMesh) 0 "/Game/Assets/LevelAssets/Buildings/Materials/MI_BuildingTexture_Casino.MI_BuildingTexture_Casino"))
    (:NewEnumerator2
      (Rendering|Material|SetMaterial (Variables|Default|GetStaticMesh) 0 "/Game/Assets/LevelAssets/Buildings/Materials/MI_BuildingTexture_Dark.MI_BuildingTexture_Dark"))
    (:NewEnumerator3
      (Rendering|Material|SetMaterial (Variables|Default|GetStaticMesh) 0 "/Game/Assets/LevelAssets/Buildings/Materials/MI_BuildingTexture_DarkBlue.MI_BuildingTexture_DarkBlue"))
    (:NewEnumerator4
      (Rendering|Material|SetMaterial (Variables|Default|GetStaticMesh) 0 "/Game/Assets/LevelAssets/Buildings/Materials/MI_BuildingTexture_DarkPurple.MI_BuildingTexture_DarkPurple"))
    (:NewEnumerator5
      (Rendering|Material|SetMaterial (Variables|Default|GetStaticMesh) 0 "/Game/Assets/LevelAssets/Buildings/Materials/MI_BuildingTexture_Gray.MI_BuildingTexture_Gray"))
    (:NewEnumerator6
      (Rendering|Material|SetMaterial (Variables|Default|GetStaticMesh) 0 "/Game/Assets/LevelAssets/Buildings/Materials/MI_BuildingTexture_Green.MI_BuildingTexture_Green"))
    (:NewEnumerator7
      (Rendering|Material|SetMaterial (Variables|Default|GetStaticMesh) 0 "/Game/Assets/LevelAssets/Buildings/Materials/MI_BuildingTexture_Light.MI_BuildingTexture_Light"))
    (:NewEnumerator8
      (Rendering|Material|SetMaterial (Variables|Default|GetStaticMesh) 0 "/Game/Assets/LevelAssets/Buildings/Materials/MI_BuildingTexture_Light2.MI_BuildingTexture_Light2"))
    (:NewEnumerator9
      (Rendering|Material|SetMaterial (Variables|Default|GetStaticMesh) 0 "/Game/Assets/LevelAssets/Buildings/Materials/MI_BuildingTexture_Red.MI_BuildingTexture_Red"))
    (:NewEnumerator10
      (Rendering|Material|SetMaterial (Variables|Default|GetStaticMesh) 0 "/Game/Assets/LevelAssets/Buildings/Materials/MI_BuildingTexture_Signs.MI_BuildingTexture_Signs"))
    (:NewEnumerator11
      (Rendering|Material|SetMaterial (Variables|Default|GetStaticMesh) 0 "/Game/Assets/LevelAssets/Buildings/Materials/MI_BuildingTexture_Yellow.MI_BuildingTexture_Yellow"))))