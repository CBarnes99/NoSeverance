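; BP_RoadDecoration is a placeable road prop that can appear as a cone, road block, road sign or speed bump.
; The construction script calls SetStaticMesh, which switches on RoadDecorationsEnum to assign the matching mesh to the StaticMesh component.
; It resets the component's world scale to one each time, then doubles it only for the speed bump.
; The event graph has no active logic.
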(event EventBeginPlay)

(event Collision|EventActorBeginOverlap
  (params (OtherActor :type Actor%20Object%20Reference)))

(event EventTick
  (params (DeltaSeconds :type Float%20%28single-precision%29)))

(fn ConstructionScript
  (CallFunction|SetStaticMesh))

(fn SetStaticMesh
  (Transformation|SetWorldScale3D (Variables|Default|GetStaticMesh) "1.000000,1.000000,1.000000")
  (switch Utilities|FlowControl|Switch|SwitchonE_RoadDecorations (Variables|Default|GetRoad%20Decorations%20Enum)
    (:NewEnumerator0
      (Components|StaticMesh|SetStaticMesh (Variables|Default|GetStaticMesh) "/Game/Assets/LevelAssets/RoadSigns/StaticMeshes/SM_Cone1.SM_Cone1"))
    (:NewEnumerator1
      (Components|StaticMesh|SetStaticMesh (Variables|Default|GetStaticMesh) "/Game/Assets/LevelAssets/RoadSigns/StaticMeshes/SM_Cone2.SM_Cone2"))
    (:NewEnumerator2
      (Components|StaticMesh|SetStaticMesh (Variables|Default|GetStaticMesh) "/Game/Assets/LevelAssets/RoadSigns/StaticMeshes/SM_RoadBlock1.SM_RoadBlock1"))
    (:NewEnumerator3
      (Components|StaticMesh|SetStaticMesh (Variables|Default|GetStaticMesh) "/Game/Assets/LevelAssets/RoadSigns/StaticMeshes/SM_RoadBlock2.SM_RoadBlock2"))
    (:NewEnumerator4
      (Components|StaticMesh|SetStaticMesh (Variables|Default|GetStaticMesh) "/Game/Assets/LevelAssets/RoadSigns/StaticMeshes/SM_RoadBlock3.SM_RoadBlock3"))
    (:NewEnumerator5
      (Components|StaticMesh|SetStaticMesh (Variables|Default|GetStaticMesh) "/Game/Assets/LevelAssets/RoadSigns/StaticMeshes/SM_RoadBlock4.SM_RoadBlock4"))
    (:NewEnumerator6
      (Components|StaticMesh|SetStaticMesh (Variables|Default|GetStaticMesh) "/Game/Assets/LevelAssets/RoadSigns/StaticMeshes/SM_RoadBlock5.SM_RoadBlock5"))
    (:NewEnumerator7
      (Components|StaticMesh|SetStaticMesh (Variables|Default|GetStaticMesh) "/Game/Assets/LevelAssets/RoadSigns/StaticMeshes/SM_RoadBlock6.SM_RoadBlock6"))
    (:NewEnumerator8
      (Components|StaticMesh|SetStaticMesh (Variables|Default|GetStaticMesh) "/Game/Assets/LevelAssets/RoadSigns/StaticMeshes/SM_RoadSign1.SM_RoadSign1"))
    (:NewEnumerator9
      (Components|StaticMesh|SetStaticMesh (Variables|Default|GetStaticMesh) "/Game/Assets/LevelAssets/RoadSigns/StaticMeshes/SM_RoadSign2.SM_RoadSign2"))
    (:NewEnumerator10
      (Components|StaticMesh|SetStaticMesh (Variables|Default|GetStaticMesh) "/Game/Assets/LevelAssets/RoadSigns/StaticMeshes/SM_RoadSign3.SM_RoadSign3"))
    (:NewEnumerator11
      (Components|StaticMesh|SetStaticMesh (Variables|Default|GetStaticMesh) "/Game/Assets/LevelAssets/RoadSigns/StaticMeshes/SM_RoadSign4.SM_RoadSign4"))
    (:NewEnumerator12
      (Components|StaticMesh|SetStaticMesh (Variables|Default|GetStaticMesh) "/Game/Assets/LevelAssets/RoadSigns/StaticMeshes/SM_SpeedBump.SM_SpeedBump")
      (Transformation|SetWorldScale3D (Variables|Default|GetStaticMesh) "2.000000,2.000000,2.000000"))))