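; BP_Nature is a placeable level-dressing actor that shows one of twelve simple nature props: variants of bushes, grass, rocks and trees.
; Its Construction Script calls SetMesh, which switches on the NatureEnum variable and assigns the matching mesh to the StaticMesh component.
; The event graph has no active logic, so the actor only picks its mesh at construction.
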(event EventBeginPlay)

(event Collision|EventActorBeginOverlap
  (params (OtherActor :type Actor%20Object%20Reference)))

(event EventTick
  (params (DeltaSeconds :type Float%20%28single-precision%29)))

(fn ConstructionScript
  (CallFunction|SetMesh))

(fn SetMesh
  (switch Utilities|FlowControl|Switch|SwitchonE_Nature (Variables|Default|GetNature%20Enum)
    (:NewEnumerator0
      (Components|StaticMesh|SetStaticMesh (Variables|Default|GetStaticMesh) "/Game/Assets/LevelAssets/SimpleNature/StaticMeshs/Bush1.Bush1"))
    (:NewEnumerator1
      (Components|StaticMesh|SetStaticMesh (Variables|Default|GetStaticMesh) "/Game/Assets/LevelAssets/SimpleNature/StaticMeshs/Bush2.Bush2"))
    (:NewEnumerator2
      (Components|StaticMesh|SetStaticMesh (Variables|Default|GetStaticMesh) "/Game/Assets/LevelAssets/SimpleNature/StaticMeshs/Bush3.Bush3"))
    (:NewEnumerator3
      (Components|StaticMesh|SetStaticMesh (Variables|Default|GetStaticMesh) "/Game/Assets/LevelAssets/SimpleNature/StaticMeshs/Grass1.Grass1"))
    (:NewEnumerator4
      (Components|StaticMesh|SetStaticMesh (Variables|Default|GetStaticMesh) "/Game/Assets/LevelAssets/SimpleNature/StaticMeshs/Grass2.Grass2"))
    (:NewEnumerator5
      (Components|StaticMesh|SetStaticMesh (Variables|Default|GetStaticMesh) "/Game/Assets/LevelAssets/SimpleNature/StaticMeshs/Grass3.Grass3"))
    (:NewEnumerator6
      (Components|StaticMesh|SetStaticMesh (Variables|Default|GetStaticMesh) "/Game/Assets/LevelAssets/SimpleNature/StaticMeshs/Rock1.Rock1"))
    (:NewEnumerator7
      (Components|StaticMesh|SetStaticMesh (Variables|Default|GetStaticMesh) "/Game/Assets/LevelAssets/SimpleNature/StaticMeshs/Rock2.Rock2"))
    (:NewEnumerator8
      (Components|StaticMesh|SetStaticMesh (Variables|Default|GetStaticMesh) "/Game/Assets/LevelAssets/SimpleNature/StaticMeshs/Rock3.Rock3"))
    (:NewEnumerator9
      (Components|StaticMesh|SetStaticMesh (Variables|Default|GetStaticMesh) "/Game/Assets/LevelAssets/SimpleNature/StaticMeshs/Tree1.Tree1"))
    (:NewEnumerator10
      (Components|StaticMesh|SetStaticMesh (Variables|Default|GetStaticMesh) "/Game/Assets/LevelAssets/SimpleNature/StaticMeshs/Tree2.Tree2"))
    (:NewEnumerator11
      (Components|StaticMesh|SetStaticMesh (Variables|Default|GetStaticMesh) "/Game/Assets/LevelAssets/SimpleNature/StaticMeshs/Tree3.Tree3"))))