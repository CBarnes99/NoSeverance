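; BP_Roads is a modular road piece actor whose shape, such as turns, full or half roads, and pavement sections, is picked through the RoadEnum variable.
; The construction script calls SetStaticMesh, which switches on the enum and assigns the matching static mesh to the RoadMesh component.
; The event graph holds only disabled default events, so the actor has no runtime logic.
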(event EventBeginPlay)

(event Collision|EventActorBeginOverlap
  (params (OtherActor :type Actor%20Object%20Reference)))

(event EventTick
  (params (DeltaSeconds :type Float%20%28single-precision%29)))

(fn ConstructionScript
  (CallFunction|SetStaticMesh))

(fn SetStaticMesh
  (switch Utilities|FlowControl|Switch|SwitchonE_Roads (Variables|Default|GetRoad%20Enum)
    (:NewEnumerator0
      (Components|StaticMesh|SetStaticMesh (Variables|Default|GetRoadMesh) "/Game/Assets/LevelAssets/Road/StaticMeshes/2Turns.2Turns"))
    (:NewEnumerator1
      (Components|StaticMesh|SetStaticMesh (Variables|Default|GetRoadMesh) "/Game/Assets/LevelAssets/Road/StaticMeshes/2TurnsCorner.2TurnsCorner"))
    (:NewEnumerator2
      (Components|StaticMesh|SetStaticMesh (Variables|Default|GetRoadMesh) "/Game/Assets/LevelAssets/Road/StaticMeshes/AllTurns.AllTurns"))
    (:NewEnumerator3
      (Components|StaticMesh|SetStaticMesh (Variables|Default|GetRoadMesh) "/Game/Assets/LevelAssets/Road/StaticMeshes/LeftTurn.LeftTurn"))
    (:NewEnumerator4
      (Components|StaticMesh|SetStaticMesh (Variables|Default|GetRoadMesh) "/Game/Assets/LevelAssets/Road/StaticMeshes/RoadFull.RoadFull"))
    (:NewEnumerator5
      (Components|StaticMesh|SetStaticMesh (Variables|Default|GetRoadMesh) "/Game/Assets/LevelAssets/Road/StaticMeshes/RoadFullLeft.RoadFullLeft"))
    (:NewEnumerator6
      (Components|StaticMesh|SetStaticMesh (Variables|Default|GetRoadMesh) "/Game/Assets/LevelAssets/Road/StaticMeshes/RoadFullNoSideWalks.RoadFullNoSideWalks"))
    (:NewEnumerator7
      (Components|StaticMesh|SetStaticMesh (Variables|Default|GetRoadMesh) "/Game/Assets/LevelAssets/Road/StaticMeshes/RoadFullRight.RoadFullRight"))
    (:NewEnumerator8
      (Components|StaticMesh|SetStaticMesh (Variables|Default|GetRoadMesh) "/Game/Assets/LevelAssets/Road/StaticMeshes/RoadHalf.RoadHalf"))
    (:NewEnumerator9
      (Components|StaticMesh|SetStaticMesh (Variables|Default|GetRoadMesh) "/Game/Assets/LevelAssets/Road/StaticMeshes/RoadHalfLeft.RoadHalfLeft"))
    (:NewEnumerator10
      (Components|StaticMesh|SetStaticMesh (Variables|Default|GetRoadMesh) "/Game/Assets/LevelAssets/Road/StaticMeshes/RoadHalfNone.RoadHalfNone"))
    (:NewEnumerator11
      (Components|StaticMesh|SetStaticMesh (Variables|Default|GetRoadMesh) "/Game/Assets/LevelAssets/Road/StaticMeshes/RoadHalfRight.RoadHalfRight"))
    (:NewEnumerator12
      (Components|StaticMesh|SetStaticMesh (Variables|Default|GetRoadMesh) "/Game/Assets/LevelAssets/Road/StaticMeshes/SideWalkFull.SideWalkFull"))
    (:NewEnumerator13
      (Components|StaticMesh|SetStaticMesh (Variables|Default|GetRoadMesh) "/Game/Assets/LevelAssets/Road/StaticMeshes/SideWalkHalf.SideWalkHalf"))))